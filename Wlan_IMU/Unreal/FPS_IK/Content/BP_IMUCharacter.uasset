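; IMU test character that visualizes motion sensor data and calibrates from a T-pose.
; Each tick, IMUReceiver data for DebugID rotates the Test component and offsets it via world-space, gravity-compensated integration, with a slight pull toward the origin against drift.
; An optional step shifts the capsule by the lower foot socket height to keep feet grounded.
; Debug keys play the T-pose before applying its configuration and toggle force feedback, while input axes move the mesh.
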(event Custom|MoveActorToGroundLEvel
  (if (Variables|Default|GetPlaceFootOnGround)
    (Utilities|FlowControl|Sequence
      (:then_0
        (bind _localpos (CallFunction|GetLocalSocketPostion "foot_lSocket")))
      (:then_1
        (bind _localpos_2 (CallFunction|GetLocalSocketPostion "foot_rSocket")))
      (:then_2
        (Transformation|SetRelativeLocation (Variables|Default|GetCapsuleComponent) (+ (Math|Vector|MakeVector 0.0 0.0 (* (select (> (.Z (Math|Vector|BreakVector _localpos)) (.Z (Math|Vector|BreakVector _localpos_2))) (.Z (Math|Vector|BreakVector _localpos_2)) (.Z (Math|Vector|BreakVector _localpos))) -1.0)) (Variables|Default|GetOffsetGround)) false false)))))

(event EventTick
  (params (DeltaSeconds :type Float%20%28single-precision%29))
  (bind _imureceiver (Variables|Default|GetIMUReceiver))
  (bind _debugid (Variables|Default|GetdebugID))
  (bind _test (Variables|Default|GetTest))
  (CallFunction|MoveActortoGroundLEvel)
  (bind _out (Class|IMUReceiver|GetRotation _imureceiver _debugid))
  (bind _returnvalue (Class|IMUReceiver|QuattoRot _imureceiver _out))
  (Transformation|SetWorldRotation _test _returnvalue false false)
  (bind _out_2 (Class|IMUReceiver|GetVelocity _imureceiver _debugid))
  (Transformation|AddWorldOffset _test (Math|Vector|Lerp(Vector) (* (* (- (Math|Vector|RotateVector _out_2 _returnvalue) "0, 0,1.000000") (- 9.8e+02 DeltaSeconds)) DeltaSeconds) (* (Transformation|GetWorldLocation _test) -2e+01) 0.0005) false false))

(event Input|AxisEvents|InputAxisMoveForward
  (params (AxisValue :type Float%20%28single-precision%29))
  (Transformation|AddWorldOffset (Variables|Character|GetMesh) (Math|Vector|MakeVector 0.0 (* AxisValue 1e+01) 0.0) false false))

(event Input|AxisEvents|InputAxisMoveRight
  (params (AxisValue :type Float%20%28single-precision%29))
  (Transformation|AddWorldRotation (Variables|Character|GetMesh) (Math|Rotator|MakeRotator 0.0 0.0 AxisValue) false false))

(event Input|KeyboardEvents|T
  (params (Key :type Key%20Structure))
  (:Pressed
    (Components|Animation|PlayAnimation (Variables|Character|GetMesh) (Variables|Default|GetTPoseAnimation) true)
    (Utilities|FlowControl|Delay 3.0)
    (Class|IMUCharacter|ApplyTPoseConfiguration)))

(event Input|KeyboardEvents|V
  (params (Key :type Key%20Structure))
  (:Pressed
    (Game|Feedback|PlayDynamicForceFeedback (Game|GetPlayerController 0) 1.0 -1.0 true true true true)))

(event Input|KeyboardEvents|B
  (params (Key :type Key%20Structure))
  (:Pressed
    (Game|Feedback|PlayDynamicForceFeedback (Game|GetPlayerController 0) 1.0 -1.0 true true true true) ; enters at Stop
  ))

(fn ConstructionScript)

(fn GetLocalSocketPostion
  (params (SocketName :type Name))
  (return (.Location (Math|Transform|BreakTransform (Transformation|GetSocketTransform (Variables|Character|GetMesh) SocketName "RTS_Component")))))