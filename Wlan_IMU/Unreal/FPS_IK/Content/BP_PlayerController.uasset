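; Player controller Blueprint that sets up the local player's UI and mouse input.
; On BeginPlay, the local controller creates a UI widget, adds it to the viewport, sets Game and UI input mode focused on it, and shows the cursor.
; Pressing R casts a valid controlled pawn to IMU_Pawn, but nothing follows the cast.
; Tick and the construction script are empty.
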(event EventBeginPlay
  (if (Pawn|IsLocalPlayerController)
    (bind _returnvalue (UserInterface|CreateWidget (Variables|Default|GetUI_Widget) self))
    (UserInterface|Viewport|AddtoViewport _returnvalue 0)
    (Input|SetInputModeGameandUI self _returnvalue "DoNotLock" false)
    (Variables|Default|SetbShowMouseCursor true)))

(event EventTick
  (params (DeltaSeconds :type Float%20%28single-precision%29)))

(event Input|KeyboardEvents|R
  (params (Key :type Key%20Structure))
  (bind _returnvalue (Pawn|GetControlledPawn))
  (:Pressed
    (Utilities|IsValid _returnvalue
      (:Is%20Valid
        (Utilities|Casting|CastToIMU_Pawn _returnvalue)))))

(fn ConstructionScript)